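; BP_Laser_Extended is a DMX-driven laser fixture that controls a Niagara laser fan effect.
; On BeginPlay it binds to its DMX component's fixture patch received event, then runs the parent's BeginPlay.
; Each received patch update sets the beam color from three attribute values, with MaxLaserIntensity as alpha.
; It also rotates the fan, centering attribute values at 0.5 and scaling them by TiltRange for pitch and PanRange for yaw.
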(event `self.ReceiveBeginPlay`
  (add `DMXComponent.OnFixturePatchReceived` (`self.DMX`) (delegate `OnFixturePatchReceived_Laser`))
  (`parent.ReceiveBeginPlay`))

(event `OnFixturePatchReceived_Laser`
  (params (FixturePatch :type "DMXEntityFixturePatch Object Reference") (ValuePerAttribute :type "DMXNormalizedAttributeValueMap Structure (by ref)"))
  (`NiagaraComponent.SetNiagaraVariableLinearColor` (`self.LaserFanVFX`) "BeamColor" (make `LinearColor` (`BlueprintMapLibrary.Map_Find` ValuePerAttribute_Map (struct :`Name` "Red")) (`BlueprintMapLibrary.Map_Find` ValuePerAttribute_Map (struct :`Name` "Green")) (`BlueprintMapLibrary.Map_Find` ValuePerAttribute_Map (struct :`Name` "Blue")) (`self.Max Laser Intensity`)))
  (`SceneComponent.K2_SetRelativeRotation` (`self.LaserFanVFX`) (`KismetMathLibrary.MakeRotator` 0.0 (* (- (`BlueprintMapLibrary.Map_Find` ValuePerAttribute_Map (struct :`Name` "Tilt")) 0.5) (`self.Tilt Range`)) (* (- (`BlueprintMapLibrary.Map_Find` ValuePerAttribute_Map (struct :`Name` "Pan")) 0.5) (`self.Pan Range`))) false false))

(fn `UserConstructionScript`
  (`parent.UserConstructionScript`))