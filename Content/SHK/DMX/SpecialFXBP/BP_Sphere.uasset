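; DMX-driven special effect sphere that floats and glows in response to fixture patch data.
; Received DMX attributes set two colors and tessellation strength in MPC_DMX_Sphere, scale the mesh, and drive point light color, intensity and radius.
; A zero check on one attribute blacks out the light.
; Each tick, three summed sine cycles, clamped, are added to the mesh's current Z position as a per-frame bobbing step.
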(event `self.ReceiveBeginPlay`
  (add `DMXComponent.OnFixturePatchReceived` (`self.DMX`) (delegate `OnFixturePatchReceived_Sphere`)))

(event `OnFixturePatchReceived_Sphere`
  (params (FixturePatch :type "DMXEntityFixturePatch Object Reference") (ValuePerAttribute :type "DMXNormalizedAttributeValueMap Structure (by ref)"))
  (bind _value (`BlueprintMapLibrary.Map_Find` ValuePerAttribute_Map (struct :`Name` "Dimmer")))
  (bind _value_2 (`BlueprintMapLibrary.Map_Find` ValuePerAttribute_Map (struct :`Name` "Zoom")))
  (bind _pointlight (`self.PointLight`))
  (bind _pointlight_2 (`self.PointLight`))
  (bind _returnvalue (`KismetMathLibrary.MapRangeUnclamped` _value_2 0.0 1.0 0.0 1.0))
  (bind _returnvalue_2 (`KismetMathLibrary.MapRangeClamped` _value 0.0 1.0 100.0 1000.0))
  (bind _linearcolor (make `LinearColor` (`BlueprintMapLibrary.Map_Find` ValuePerAttribute_Map (struct :`Name` "Red")) (`BlueprintMapLibrary.Map_Find` ValuePerAttribute_Map (struct :`Name` "Green")) (`BlueprintMapLibrary.Map_Find` ValuePerAttribute_Map (struct :`Name` "Blue"))))
  (`KismetMaterialLibrary.SetVectorParameterValue` "/Game/SHK/DMX/FixtureMaterials/MPC_DMX_Sphere.MPC_DMX_Sphere" "Color1" _linearcolor)
  (`KismetMaterialLibrary.SetVectorParameterValue` "/Game/SHK/DMX/FixtureMaterials/MPC_DMX_Sphere.MPC_DMX_Sphere" "Color2" (make `LinearColor` (`BlueprintMapLibrary.Map_Find` ValuePerAttribute_Map (struct :`Name` "Cyan")) (`BlueprintMapLibrary.Map_Find` ValuePerAttribute_Map (struct :`Name` "Magenta")) (`BlueprintMapLibrary.Map_Find` ValuePerAttribute_Map (struct :`Name` "Yellow"))))
  (`KismetMaterialLibrary.SetScalarParameterValue` "/Game/SHK/DMX/FixtureMaterials/MPC_DMX_Sphere.MPC_DMX_Sphere" "TessStrength" _value)
  (`SceneComponent.SetWorldScale3D` (`self.StaticMesh`) (* (`KismetMathLibrary.MakeVector` 4.0 4.0 4.0) (`KismetMathLibrary.Conv_DoubleToVector` _value_2)))
  (if (== _value_2 0.0)
    (`LightComponent.SetLightColor` :`self` _pointlight_2)
    (`LightComponent.SetIntensity` _pointlight_2 0.0)
    (`LocalLightComponent.SetAttenuationRadius` _pointlight_2 0.0)
    (else
      (`LightComponent.SetLightColor` _pointlight _linearcolor true)
      (`LightComponent.SetIntensity` _pointlight (+ (`self.MinInt`) (* (* _returnvalue_2 _returnvalue) (`self.IntMult`))))
      (`LocalLightComponent.SetAttenuationRadius` _pointlight (+ (`self.MinRange`) (* _returnvalue_2 _returnvalue))))))

(event `self.ReceiveTick`
  (params (DeltaSeconds :type "Float (single-precision)"))
  (bind _returnvalue (* (`GameplayStatics.GetWorldDeltaSeconds`) 360.0))
  ;[1 1 1] Tick floating movement
  (`|ExecutionSequence`
    (:`then_0`
      (set `self.BobbingCycle1` (mod (+ (/ _returnvalue (`self.BobbingPeriod1`)) (`self.BobbingCycle1`)) 360.0)))
    (:`then_1`
      (set `self.BobbingCycle2` (mod (+ (/ _returnvalue (`self.BobbingPeriod2`)) (`self.BobbingCycle2`)) 360.0)))
    (:`then_2`
      (set `self.BobbingCycle3` (mod (+ (/ _returnvalue (`self.BobbingPeriod3`)) (`self.BobbingCycle3`)) 360.0)))
    (:`then_3`
      (`SceneComponent.K2_SetRelativeLocation` (`self.StaticMesh`) (+ (`SceneComponent.RelativeLocation` (`self.StaticMesh`)) (`KismetMathLibrary.MakeVector` 0.0 0.0 (`KismetMathLibrary.FClamp` (+ (* (`self.BobbingAmplitude1`) (`KismetMathLibrary.DegSin` (`self.BobbingCycle1`))) (* (`self.BobbingAmplitude2`) (`KismetMathLibrary.DegSin` (`self.BobbingCycle2`))) (* (`self.BobbingAmplitude3`) (`KismetMathLibrary.DegSin` (`self.BobbingCycle3`)))) -100.0 10000.0))) false false))))

(fn `UserConstructionScript`)