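; BP_TrafficLight is an actor that plays selectable music and spawns random note actors in response to the track's cues.
; Custom events choose a sound from the Music array and activate or deactivate the audio component.
; PlayMusic watches the MetaSound output "AstroCue", and each change spawns a random class from NoteClasses at the arrow component's location and rotation.
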(event `Stop Music`
  ;[1 1 1] Music Start, Stop Trigger
  (`ActorComponent.SetActive` (`self.AudioComp`) false false))

(event `self.ReceiveBeginPlay`
  ;[1 1 1] Music Start
)

(event `Play Music`
  (bind _audiocomp (`self.AudioComp`))
  ;[1 1 1] Music Start
  (`ActorComponent.SetActive` _audiocomp true false)
  (`MetaSoundOutputSubsystem.WatchOutput` (subsystem `MetaSoundOutputSubsystem`) _audiocomp "AstroCue" (delegate `CueChange`) "None" "None"))

(event `CueChange`
  (params (OutputName :type Name) (Output :type "MetaSoundOutput Structure (by ref)"))
  (bind _arrowcomp (`self.ArrowComp`))
  ;[1 1 1] Music Start
  (`|SpawnActorFromClass` (`KismetArrayLibrary.Array_Random` (`self.NoteClasses`)) (`KismetMathLibrary.MakeTransform` (`SceneComponent.K2_GetComponentLocation` _arrowcomp) (`SceneComponent.K2_GetComponentRotation` _arrowcomp)) "Undefined" "MultiplyWithRoot" null null))

(event `Set Music`
  (params (Index :type Integer))
  ;[1 1 1] Set Music
  (`AudioComponent.SetSound` (`self.AudioComp`) (`|GetArrayItem` (`self.Music`) Index)))

(fn `UserConstructionScript`)