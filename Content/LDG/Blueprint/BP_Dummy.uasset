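; BP_Dummy is a controller Blueprint that lets microphone or captured audio volume raise and lower the level's BP_HitTool.
; On BeginPlay it finds the hit tool and the BP_TrafficLight, which serves as the music box.
; Each audio envelope update nudges the tool's height, sinking slightly when quiet and rising when louder, up to a ceiling.
; R toggles the music, and holding right mouse enables the tool's hit collision for queries.
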(event `self.ReceiveBeginPlay`
  (`|ExecutionSequence`
    (:`then_0`
      (bind _returnvalue (`GameplayStatics.GetActorOfClass` "/Game/LDG/Blueprint/BP_HitTool.BP_HitTool_C"))
      (set `self.HitTool` _returnvalue)
      (bind _returnvalue_2 (`GameplayStatics.GetActorOfClass` "/Game/LDG/Blueprint/BP_TrafficLight.BP_TrafficLight_C"))
      (set `self.MusicBox` _returnvalue_2))))

(event `self.AudioCapture.OnAudioEnvelopeValue`
  (params (EnvelopeValue :type "Float (single-precision)"))
  (bind (_returnvalue_x _returnvalue_y _returnvalue_z) (`KismetMathLibrary.BreakVector` (`self.K2_GetActorLocation` (`self.HitTool`))))
  (bind _returnvalue (+ _returnvalue_z (`KismetMathLibrary.MapRangeClamped` EnvelopeValue 0.0 1.0 -1.0 50.0)))
  (if (>= _returnvalue 400.0)
    (set `self.ElavateValue` 400.0)
    (else
      (set `self.ElavateValue` _returnvalue)))
  (`SceneComponent.K2_SetWorldLocation` (`Actor.RootComponent` (`self.HitTool`)) (`KismetMathLibrary.MakeVector` _returnvalue_x _returnvalue_y (`self.ElavateValue`)) false false))

(event `Key|R`
  (params (Key :type "Key Structure"))
  (bind _musicbox (`self.MusicBox`))
  (:`Pressed`
    (`/Engine/EditorBlueprintResources/StandardMacros.FlipFlop`
      (:`A`
        (`/Game/LDG/Blueprint/BP_TrafficLight.Play Music` _musicbox))
      (:`B`
        (`/Game/LDG/Blueprint/BP_TrafficLight.Stop Music` _musicbox)))))

(event `Key|RightMouseButton`
  (params (Key :type "Key Structure"))
  (bind _hitcollision (`HitTool.HitCollision` (`self.HitTool`)))
  (:`Pressed`
    (`PrimitiveComponent.SetCollisionEnabled` _hitcollision "QueryOnly"))
  (:`Released`
    (`PrimitiveComponent.SetCollisionEnabled` _hitcollision "NoCollision")))

(event `Key|One`
  (params (Key :type "Key Structure")))

(fn `UserConstructionScript`)