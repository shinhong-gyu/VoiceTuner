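; Game manager for a music game that handles song selection, the play timer and game end.
; SetCurrentSong creates the main UI with art and title and passes the index to the player character's Setmusic; CancleSong resets the selection.
; While playing, Tick accumulates time and calls the character's GameEnd at 211 seconds, as does stopgame immediately.
; The server-to-multicast song event ends in an empty handler, and timed recording calls are disconnected.
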(event `self.ReceiveBeginPlay`
  (bind _returnvalue (`GameplayStatics.GetActorOfClass` "/Game/LDG/Blueprint/BP_TrafficLight.BP_TrafficLight_C"))
  (set `self.NoteSpawner` _returnvalue))

(event `stop game`
  (set `self.IsPlaying` false)
  (bind _asbp_hsw_third_person_character (cast `/Game/HSW/ThirdPerson/Blueprints/BP_HSW_ThirdPersonCharacter` (`GameplayStatics.GetPlayerPawn` 0)))
  (`/Game/HSW/ThirdPerson/Blueprints/BP_HSW_ThirdPersonCharacter.GameEnd` _asbp_hsw_third_person_character))

(event `ServerSetCurrentSong`
  (params (NewParam :type "AudioComponent Object Reference") (NewParam2 :type "Texture2D Object Reference") (NewParam3 :type String) (NewParam4 :type Integer))
  (`self.MultiSetCurrentSong` NewParam NewParam2 NewParam3 NewParam4))

(event `SetCurrentSong`
  (params (CurrentSong :type "AudioComponent Object Reference") (Image :type "Texture2D Object Reference") (SingerSongName :type String) (Index :type Integer))
  (set `self.CurrentSong` CurrentSong)
  (bind _returnvalue (`|CreateWidget` "/Game/HSW/UI/WBP_MainUI.WBP_MainUI_C"))
  (bind _output_get (set `self.MainUI` _returnvalue))
  (`UserWidget.AddToViewport` _output_get 0)
  (`Image.SetBrushFromTexture` (`/Game/HSW/UI/WBP_MainUI.CurrentSongImage` (`self.MainUI`)) Image false)
  (set `TextBlock.Text` (`KismetTextLibrary.Conv_StringToText` SingerSongName) (`/Game/HSW/UI/WBP_MainUI.SongTitle` (`self.MainUI`)))
  (`Widget.SetVisibility` (`/Game/HSW/UI/WBP_MainUI.CancelButton` (`self.MainUI`)) "Visible")
  (bind _output_get_2 (set `self.songindex` Index))
  (bind _asbp_hsw_third_person_character (cast `/Game/HSW/ThirdPerson/Blueprints/BP_HSW_ThirdPersonCharacter` (`GameplayStatics.GetPlayerPawn` 0)))
  (`/Game/HSW/ThirdPerson/Blueprints/BP_HSW_ThirdPersonCharacter.setmusic` _asbp_hsw_third_person_character _output_get_2))

(event `MultiSetCurrentSong`
  (params (NewParam :type "AudioComponent Object Reference") (NewParam2 :type "Texture2D Object Reference") (NewParam3 :type String) (NewParam4 :type Integer)))

(event `CancleSong`
  (`Widget.SetVisibility` (`/Game/HSW/UI/WBP_MainUI.CancelButton` (`self.MainUI`)) "Hidden")
  (set `self.CurrentSong` null)
  (`Image.SetBrushFromTexture` (`/Game/HSW/UI/WBP_MainUI.CurrentSongImage` (`self.MainUI`)) "/Engine/EditorLandscapeResources/DefaultAlphaTexture.DefaultAlphaTexture" false)
  (set `TextBlock.Text` "None" (`/Game/HSW/UI/WBP_MainUI.SongTitle` (`self.MainUI`))))

(event `self.ReceiveTick`
  (params (DeltaSeconds :type "Float (single-precision)"))
  (bind _playingtime (`self.PlayingTime`))
  (if (`self.IsPlaying`)
    (set `self.PlayingTime` (+ (`self.PlayingTime`) DeltaSeconds))
    (if (and (>= _playingtime 50.0) (< _playingtime 66.7) (not (`self.RecordStart`)))
      _
      (elif (and (>= (`self.PlayingTime`) 66.7) (`self.RecordStart`))
        _
        (elif (>= (`self.PlayingTime`) 211.0)
          (set `self.PlayingTime` 0.0)
          (set `self.IsPlaying` false)
          (bind _asbp_hsw_third_person_character (cast `/Game/HSW/ThirdPerson/Blueprints/BP_HSW_ThirdPersonCharacter` (`GameplayStatics.GetPlayerPawn` 0)))
          (`/Game/HSW/ThirdPerson/Blueprints/BP_HSW_ThirdPersonCharacter.GameEnd` _asbp_hsw_third_person_character))))))

(fn `UserConstructionScript`)